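; GM_LeaveMeAllone is a game mode that runs a countdown timer for the match.
; On BeginPlay a looping one-second timer decrements GameTime.
; When GameTime reaches zero, the timer is cleared and the first player controller is cast to PC_LeaveMeAlone, with no logic following the cast.
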(event `self.ReceiveBeginPlay`
  (bind _returnvalue (`KismetSystemLibrary.K2_SetTimerDelegate` (delegate `GameTimer`) 1.0 true))
  (set `self.GameTimerHandle` _returnvalue))

(event `GameTimer`
  (bind _output_get (set `self.GameTime` (- (`self.GameTime`) 1)))
  (if (== _output_get 0)
    (`|ExecutionSequence`
      (:`then_0`
        (`KismetSystemLibrary.K2_ClearAndInvalidateTimerHandle` (`self.GameTimerHandle`)))
      (:`then_1`
        (cast `/Game/LeaveMeAlone/Core/Controller/PC_LeaveMeAlone` (`GameplayStatics.GetPlayerController` 0))))))

(fn `UserConstructionScript`)